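; Gameplay Ability for BP_ArkdChar that performs the Shocking Grass attack through the character's melee sphere.
; On activation it activates the sphere and commits, then plays AM_ShockingGrass with query collision enabled on the sphere.
; Any montage exit disables collision and ends the ability, and OnEndAbility switches off MeleeParticles.
; A failed commit has no EndAbility call, and hit handling is not in this graph.
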(event Ability|EventActivateAbility
  (bind _asbp_arkd_char (Utilities|Casting|CastToBP_ArkdChar (.OwnerActor (Utilities|Struct|BreakGameplayAbilityActorInfo (Ability|GetActorInfo)))))
  (bind _output_get (Variables|Default|SetAs%20BP%20Arkd%20Char _asbp_arkd_char))
  (Components|Activation|Activate (Variables|/Game/BP/Character/BP_ArkdChar.BP_ArkdChar_C|GetMeleeSphere _output_get) false)
  (bind _returnvalue (Ability|CommitAbility))
  (if _returnvalue
    (|PlayMontageandWaitProxy "None" "/Game/retargetAnim/AM_ShockingGrass.AM_ShockingGrass" 1.0 "None" true 1.0 0.0
      (:then
        (Collision|SetCollisionEnabled (Variables|/Game/BP/Character/BP_ArkdChar.BP_ArkdChar_C|GetMeleeSphere (Variables|Default|GetAs%20BP%20Arkd%20Char)) "QueryOnly"))
      (:OnCompleted
        (Collision|SetCollisionEnabled (Variables|/Game/BP/Character/BP_ArkdChar.BP_ArkdChar_C|GetMeleeSphere (Variables|Default|GetAs%20BP%20Arkd%20Char)) "NoCollision" :!label _label)
        (Ability|EndAbility))
      (:OnBlendOut
        (goto _label))
      (:OnInterrupted
        (goto _label))
      (:OnCancelled
        (goto _label)))))

(event Ability|EventOnEndAbility
  (params (bWasCancelled :type Boolean))
  (Components|Activation|SetActive (Variables|/Game/BP/Character/BP_ArkdChar.BP_ArkdChar_C|GetMeleeParticles (Variables|Default|GetAs%20BP%20Arkd%20Char)) false false))