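; Gameplay Ability that casts a firebolt from the Arkd character with a cast montage.
; After committing, it plays the montage and spawns a projectile attached to the ability socket on the character.
; A montage notify detaches the projectile and launches it along the character's forward vector at the projectile speed.
; The ability ends when the montage completes, blends out or is interrupted, and cancels if the cast or commit fails.
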(event Ability|EventActivateAbility
  (bind _asbp_arkd_char (Utilities|Casting|CastToBP_ArkdChar (.OwnerActor (Utilities|Struct|BreakGameplayAbilityActorInfo (Ability|GetActorInfo))))
    (:then
      (Variables|Default|SetAs%20BP%20Arkd%20Char _asbp_arkd_char)
      (bind _returnvalue (Ability|CommitAbility))
      (if _returnvalue
        (Animation|Montage|PlayMontage (Variables|/Script/Engine.Character|GetMesh (Variables|Default|GetAs%20BP%20Arkd%20Char)) "/Game/retargetAnim/AM_CastFireBolt.AM_CastFireBolt"
          (:then
            (bind _spawnedactor (|SpawnActor :Class "/Game/BP/Abilities/Firebolt/BP_AcmProjectile.BP_AcmProjectile_C" :Instigator (Variables|Default|GetAs%20BP%20Arkd%20Char))
              (:Success
                (bind _asbp_acm_projectile (Utilities|Casting|CastToBP_AcmProjectile _spawnedactor))
                (bind _output_get (Variables|Default|SetAs%20BP%20Acm%20Projectile _asbp_acm_projectile))
                (Transformation|AttachActorToActor _output_get (Variables|Default|GetAs%20BP%20Arkd%20Char) "AbilityRightSocket" "KeepRelative" "KeepRelative" "KeepRelative" true))))
          (:OnCompleted
            (Ability|EndAbility :!label _label))
          (:OnBlendOut
            (goto _label))
          (:OnInterrupted
            (goto _label))
          (:OnNotifyBegin
            (bind _as_bp_acm_projectile (Variables|Default|GetAs%20BP%20Acm%20Projectile)
              (:then
                (Transformation|DetachFromActor _as_bp_acm_projectile "KeepRelative" "KeepRelative" "KeepRelative")
                (Default|InitProjectileMovement (Variables|Default|GetAs%20BP%20Acm%20Projectile) (* (Transformation|GetActorForwardVector (Variables|Default|GetAs%20BP%20Arkd%20Char)) (Variables|Default|GetProjectileSpeed))))
              (:else))))
        (else
          (Ability|CancelAbility :!label _label_2))))
    (:CastFailed
      (goto _label_2))))

(event Ability|EventOnEndAbility
  (params (bWasCancelled :type Boolean)))