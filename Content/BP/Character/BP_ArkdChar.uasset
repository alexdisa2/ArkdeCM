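; Player character Blueprint using the Gameplay Ability System, with mana regeneration and a life-stealing melee touch.
; BeginPlay attaches the melee sphere to a left-hand ability socket, applies mana regen, and feeds the AttributeSet to the stats widget, destroying that component when not locally controlled.
; Overlapping another BP_ArkdChar with the sphere activates particles and applies ShockingGrass damage to the target and healing to itself.
; End overlap has no effect.
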(event OnComponentBeginOverlap(MeleeSphere)
  (params (OverlappedComponent :type Primitive%20Component%20Object%20Reference) (OtherActor :type Actor%20Object%20Reference) (OtherComp :type Primitive%20Component%20Object%20Reference) (OtherBodyIndex :type Integer) (bFromSweep :type Boolean) (SweepResult :type Hit%20Result%20Structure%20%28by%20ref%29))
  (bind _asbp_arkd_char (Utilities|Casting|CastToBP_ArkdChar OtherActor))
  (if (!= _asbp_arkd_char self)
    (Components|Activation|SetActive (Variables|Default|GetMeleeParticles) true false)
    (GameplayEffects|ApplyGameplayEffectToSelf :self (Variables|/Script/ArkdeCM.ArkdeCMCharacter|GetAbilitySystemComponenet _asbp_arkd_char) :GameplayEffectClass "/Game/BP/Abilities/ShockingGrass/GE_ShockingGrassDamage.GE_ShockingGrassDamage_C")
    (GameplayEffects|ApplyGameplayEffectToSelf :self (Variables|Default|GetAbilitySystemComponenet) :GameplayEffectClass "/Game/BP/Abilities/ShockingGrass/GE_ShockingGrassHeal.GE_ShockingGrassHeal_C")))

(event OnComponentEndOverlap(MeleeSphere)
  (params (OverlappedComponent :type Primitive%20Component%20Object%20Reference) (OtherActor :type Actor%20Object%20Reference) (OtherComp :type Primitive%20Component%20Object%20Reference) (OtherBodyIndex :type Integer))
  (bind _asbp_arkd_char (Utilities|Casting|CastToBP_ArkdChar OtherActor))
  (if (!= _asbp_arkd_char self)
    _))

(event EventBeginPlay
  (bind _wc_stats (Variables|Default|GetWC_Stats))
  (Transformation|AttachComponentToComponent (Variables|Default|GetMeleeSphere) (Variables|Character|GetMesh) "AbilityLeftSocket" "KeepRelative" "KeepRelative" "KeepRelative" true)
  (GameplayEffects|ApplyGameplayEffectToSelf :self (Variables|Default|GetAbilitySystemComponenet) :GameplayEffectClass "/Game/BP/GameplayEffects/GE_ManaRegen.GE_ManaRegen_C")
  ;[1 1 1] control local del widget de en pantalla
  (if (Pawn|IsLocallyControlled)
    (bind _aswbp_stats (Utilities|Casting|CastToWBP_Stats (UserInterface|GetUserWidgetObject _wc_stats)))
    (Variables|/Game/BP/WBP/WBP_Stats.WBP_Stats_C|SetAttributeSet _aswbp_stats (Variables|Default|GetAttributeSet))
    (else
      (Components|DestroyComponent _wc_stats))))

(event Collision|EventActorBeginOverlap
  (params (OtherActor :type Actor%20Object%20Reference)))

(event EventTick
  (params (DeltaSeconds :type Float%20%28single-precision%29)))

(fn ConstructionScript)